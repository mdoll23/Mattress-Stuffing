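; BP_PickupMaster is a pickup actor that adds an item to the inventory when the top-down character overlaps it.
; On overlap with BP_TopDownCharacter, it adds its Type to the Inventory held on the custom Game Instance, then destroys itself.
; The Construction Script applies the PickupMesh and Material variables to the mesh component, so each pickup's look comes from its variables.
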(event Collision|EventActorBeginOverlap
  (params (OtherActor :type Actor%20Object%20Reference))
  (Utilities|Casting|CastToBP_TopDownCharacter OtherActor)
  (bind _asgame_instance_custom (Utilities|Casting|CastToGameInstance_Custom (Game|GetGameInstance)))
  (Utilities|Array|Add (Variables|/Game/Inventory/GameInstance_Custom.GameInstance_Custom_C|GetInventory _asgame_instance_custom) (Variables|Default|GetType))
  (Actor|DestroyActor))

(fn ConstructionScript
  (Components|StaticMesh|SetStaticMesh (Variables|Default|Getmesh) (Variables|Default|GetPickupMesh))
  (Rendering|Material|SetMaterial (Variables|Default|Getmesh) 0 (Variables|Default|GetMaterial)))