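; Actor component for talkable actors that runs data-table-driven dialogue and toggles a custom depth stencil highlight on the mesh.
; DialogueInteract creates the overworld dialogue widget or updates it, following each row's next row and table until an end flag closes it.
; Open-ended choices, built only at widget creation, show the cursor and spawn option widgets referencing the component.
; Option_Selected jumps to a chosen row; LeaveDialogue restores game-only input.
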(event Custom|Option_Selected
  (params (RowName :type Name) (DataTable :type Data%20Table%20Object%20Reference))
  (bind _dialogue_widget (Variables|Default|Getdialogue_Widget))
  (bind _returnvalue (Utilities|GetDataTableRow DataTable RowName)
    (:then
      (Widget|Panel|ClearChildren (Variables|/Game/Dialogue_System_Prototype/UI_Overworld_Dialogue.UI_Overworld_Dialogue_C|GetOption_ScrollBox _dialogue_widget))
      (Default|UpdateDialogue _dialogue_widget (.Dialogue (Utilities|Struct|BreakBP_Dialogue_Structure _returnvalue)))
      (Variables|Default|SetRow%20Name (.Row (Utilities|Struct|BreakBP_Dialogue_Structure _returnvalue)))
      (Variables|Default|SetData_Table (.DataTable (Utilities|Struct|BreakBP_Dialogue_Structure _returnvalue)))
      (Variables|Default|Setend_Dialogue (.EndDialogue? (Utilities|Struct|BreakBP_Dialogue_Structure _returnvalue))))))

(event EventHighlightActor
  (params (Actor_Ref :type Actor%20Object%20Reference) (Active? :type Boolean))
  (bind _returnvalue (Actor|GetComponentbyClass Actor_Ref "/Script/Engine.MeshComponent"))
  ;[0 1 0.1142] Highlight actor when in teraction range
  (Rendering|SetRenderCustomDepth _returnvalue (Variables|Default|GetdefaultCustomDepthPass?))
  (if Active?
    (Rendering|SetRenderCustomDepth _returnvalue true)
    (Rendering|SetCustomDepthStencilValue _returnvalue 5)
    (else
      (Rendering|SetCustomDepthStencilValue _returnvalue 0))))

(event EventDialogueInteract
  (params (player_ref :type BP%20Top%20Down%20Character%20Object%20Reference))
  (bind _returnvalue (Game|GetPlayerController 0))
  (bind _returnvalue_2 (Game|GetPlayerController 0))
  (if (Variables|Default|Getend_Dialogue)
    (Widget|RemovefromParent (Variables|Default|Getdialogue_Widget))
    (Variables|Default|Setend_Dialogue false)
    (Variables|Default|Setdialogue_Widget 0)
    (Input|SetInputModeGameOnly _returnvalue false)
    (Variables|/Script/Engine.PlayerController|SetbShowMouseCursor _returnvalue false)
    (else
      (Utilities|IsValid (Variables|Default|Getdialogue_Widget)
        (:Is%20Valid
          (bind _returnvalue_3 (Utilities|GetDataTableRow (Variables|Default|GetData_Table) (Variables|Default|GetRow%20Name))
            (:then
              (Default|UpdateDialogue (Variables|Default|Getdialogue_Widget) (.Dialogue (Utilities|Struct|BreakBP_Dialogue_Structure _returnvalue_3)))
              (Variables|Default|SetRow%20Name (.Row (Utilities|Struct|BreakBP_Dialogue_Structure _returnvalue_3)))
              (Variables|Default|SetData_Table (.DataTable (Utilities|Struct|BreakBP_Dialogue_Structure _returnvalue_3)))
              (Variables|Default|Setend_Dialogue (.EndDialogue? (Utilities|Struct|BreakBP_Dialogue_Structure _returnvalue_3))))))
        (:Is%20Not%20Valid
          (bind _returnvalue_4 (Utilities|GetDataTableRow (Variables|Default|GetData_Table) (Variables|Default|GetRow%20Name))
            (:then
              (bind _returnvalue_5 (UserInterface|CreateWidget "/Game/Dialogue_System_Prototype/UI_Overworld_Dialogue.UI_Overworld_Dialogue_C" 0 (Utilities|Text|ToText(Name) (Variables|Default|GetName)) (.Dialogue (Utilities|Struct|BreakBP_Dialogue_Structure _returnvalue_4))))
              (bind _output_get (Variables|Default|Setdialogue_Widget _returnvalue_5))
              (UserInterface|Viewport|AddtoViewport _output_get 0)
              (Variables|Default|SetRow%20Name (.Row (Utilities|Struct|BreakBP_Dialogue_Structure _returnvalue_4)))
              (Variables|Default|SetData_Table (.DataTable (Utilities|Struct|BreakBP_Dialogue_Structure _returnvalue_4)))
              (Variables|Default|Setend_Dialogue (.EndDialogue? (Utilities|Struct|BreakBP_Dialogue_Structure _returnvalue_4)))
              (if (.OpenEndedDialogue? (Utilities|Struct|BreakBP_Dialogue_Structure _returnvalue_4))
                (Input|SetInputModeGameandUI _returnvalue_2 0 "DoNotLock" true false)
                (Variables|/Script/Engine.PlayerController|SetbShowMouseCursor _returnvalue_2 true)
                (for _array_element (.OpenEndedDialogueOptions (Utilities|Struct|BreakBP_Dialogue_Structure _returnvalue_4))
                  (bind _returnvalue_6 (UserInterface|CreateWidget "/Game/Dialogue_System_Prototype/UI_Dialogue_Options.UI_Dialogue_Options_C" 0 (Utilities|Text|ToText(Name) (.option_Name (Utilities|Struct|BreakBP_Options_Dialogue_Structure _array_element))) self (.Row (Utilities|Struct|BreakBP_Options_Dialogue_Structure _array_element)) (.Data_Table (Utilities|Struct|BreakBP_Options_Dialogue_Structure _array_element))))
                  (Widget|Panel|AddChild (Variables|/Game/Dialogue_System_Prototype/UI_Overworld_Dialogue.UI_Overworld_Dialogue_C|GetOption_ScrollBox (Variables|Default|Getdialogue_Widget)) _returnvalue_6))))))))))

(event EventBeginPlay
  (bind _self self)
  (bind _returnvalue (Components|GetOwner _self))
  (bind _returnvalue_2 (Actor|GetComponentbyClass _returnvalue "/Script/Engine.MeshComponent"))
  ;[0.02587 0.4469 0] Is Default Custom Depth Pass Enabled?
  (if (Variables|Default|GetdefaultCustomDepthPass?)
    (Rendering|SetRenderCustomDepth _returnvalue_2 true)
    (else
      (Rendering|SetRenderCustomDepth _returnvalue_2 false))))

(event EventLeaveDialogue
  (bind _returnvalue (Game|GetPlayerController 0))
  ;[0 1 0.1724] Player walks away
  (Utilities|IsValid (Variables|Default|Getdialogue_Widget)
    (:Is%20Valid
      (Widget|RemovefromParent (Variables|Default|Getdialogue_Widget))
      (Variables|Default|Setend_Dialogue false)
      (Variables|Default|Setdialogue_Widget 0)
      (Input|SetInputModeGameOnly _returnvalue false)
      (Variables|/Script/Engine.PlayerController|SetbShowMouseCursor _returnvalue false))))